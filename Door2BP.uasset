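; Interactive door Blueprint that the player opens and closes with the E key while standing near it.
; A box trigger enables input for player controller 0 on overlap and disables it when the overlap ends.
; Each press toggles OpeningDoor, playing or reversing a timeline whose tracks drive door yaw and handle roll through Lerps.
; The handle only animates while the door is opening.
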(event `Key|E`
  (params (Key :type "Key Structure"))
  (:`Pressed`
    (bind _output_get (set `self.Opening Door` (not (`self.Opening Door`))))
    (if _output_get
      (bind (_direction _door_handle _door) (`Timeline|Timeline_0` :!label _label)
        (:`Update`
          (`SceneComponent.K2_SetRelativeRotation` (`self.door`) (`KismetMathLibrary.MakeRotator` 0.0 0.0 (`KismetMathLibrary.Lerp` 0.0 110.0 _door)) false false)
          (if (`self.Opening Door`)
            (`SceneComponent.K2_SetRelativeRotation` (`self.Handle2`) (`KismetMathLibrary.MakeRotator` (`KismetMathLibrary.Lerp` 0.0 40.0 _door_handle)) false false))))
      (else
        (goto _label :!via `Reverse`)))))

(event `self.Box.OnComponentBeginOverlap`
  (params (OverlappedComponent :type "PrimitiveComponent Object Reference") (OtherActor :type "Actor Object Reference") (OtherComp :type "PrimitiveComponent Object Reference") (OtherBodyIndex :type Integer) (bFromSweep :type Boolean) (SweepResult :type "HitResult Structure (by ref)"))
  (`self.EnableInput` (`GameplayStatics.GetPlayerController` 0)))

(event `self.Box.OnComponentEndOverlap`
  (params (OverlappedComponent :type "PrimitiveComponent Object Reference") (OtherActor :type "Actor Object Reference") (OtherComp :type "PrimitiveComponent Object Reference") (OtherBodyIndex :type Integer))
  (`self.DisableInput` (`GameplayStatics.GetPlayerController` 0)))

(fn `UserConstructionScript`)